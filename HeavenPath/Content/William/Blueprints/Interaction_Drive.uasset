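; Interactable steering control that turns the shared Angle value in BP_GameMode left or right, as set by its IsRight flag.
; UsingObject caches the game mode and opens a gate, and UnUsing closes it.
; Tick feeds that gate once the left mouse button is held briefly, so AngleCalcule steps Angle by RotationPower every frame within a clamped range, without delta-time scaling.
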(event EventTick
  (params (DeltaSeconds :type Float%20%28single-precision%29))
  (|CallParentFunction DeltaSeconds)
  (if (>= (Class|PlayerController|GetInputKeyTimeDown (Game|GetPlayerController 0) "LeftMouseButton") 0.16)
    (Utilities|FlowControl|Gate true
      (:Exit
        (CallFunction|AngleCalcule (Variables|Default|GetIsRight))))))

(event EventUsingObject
  (bind _asbp_game_mode (Utilities|Casting|CastToBP_GameMode (Game|GetGameMode)))
  (Variables|Default|SetGameMode _asbp_game_mode)
  (Utilities|FlowControl|Gate true) ; enters at Open
)

(event EventUnUsing
  (Utilities|FlowControl|Gate true) ; enters at Close
)

(fn ConstructionScript
  (|CallParentFunction))

(fn AngleCalcule
  (params (Isright :type Boolean))
  (bind _gamemode (Variables|Default|GetGameMode))
  (bind _gamemode_2 (Variables|Default|GetGameMode))
  (if Isright
    (Variables|/Game/William/Blueprints/Player/BP_GameMode.BP_GameMode_C|SetAngle _gamemode (Math|Float|Clamp(Float) (+ (Variables|/Game/William/Blueprints/Player/BP_GameMode.BP_GameMode_C|GetAngle _gamemode) (Variables|/Game/William/Blueprints/Player/BP_GameMode.BP_GameMode_C|GetRotationPower _gamemode)) -45.0 45.0))
    (else
      (Variables|/Game/William/Blueprints/Player/BP_GameMode.BP_GameMode_C|SetAngle _gamemode_2 (Math|Float|Clamp(Float) (- (Variables|/Game/William/Blueprints/Player/BP_GameMode.BP_GameMode_C|GetAngle _gamemode_2) (Variables|/Game/William/Blueprints/Player/BP_GameMode.BP_GameMode_C|GetRotationPower _gamemode_2)) -45.0 45.0)))))