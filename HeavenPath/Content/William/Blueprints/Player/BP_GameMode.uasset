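; Game mode that tracks a left/right drift score driven by an angle and drains player HP when it strays too far.
; Each Tick maps Angle to a clamped point rate and adds it to a bounded running total.
; In either outer band, a Delay throttles an alert sound and HP loss to about once per second.
; DangerEditor, a randomised danger-range check with debug direction prints, is never executed.
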(event Custom|LostHP
  ;[1 1 1] Subit des dégâts
  (if (not (<= (Variables|Default|GetHP) 0.0))
    (Variables|Default|SetHP (- (Variables|Default|GetHP) 1.0))))

(event EventTick
  (params (DeltaSeconds :type Float%20%28single-precision%29))
  (bind _rangepoint_s (Variables|Default|GetRangePoint/s))
  ;[1 1 1] Calcule des points par secondes
  (Variables|Default|SetPoint/S (Math|Integer|Clamp(Integer) (Math|Float|Truncate (Math|Float|Lerp _rangepoint_s (* _rangepoint_s -1.0) (Math|Float|NormalizetoRange (Variables|Default|GetAngle) -45.0 45.0))) -10 10))
  (bind _output_get (Variables|Default|SetPoint (Math|Integer|Clamp(Integer) (+ (Variables|Default|GetPoint/S) (Variables|Default|GetPoint)) -200 200)))
  ;[1 1 1] Si il touche les murs prend des dégâts
  (if (or (Math|Integer|InRange(Integer) _output_get -200 -100) (Math|Integer|InRange(Integer) _output_get 100 200))
    (Utilities|FlowControl|Delay 1.0)
    (Audio|PlaySound2D "/Game/William/Blueprints/AlerteDirectionV1wav.AlerteDirectionV1wav")
    (CallFunction|LostHP)))

(fn ConstructionScript)

(fn DangerEditor
  (params (Point :type Integer))
  (if (> (Variables|Default|GetAngle) 0.0)
    (Development|PrintString "Droite")
    (else
      (Development|PrintString "gauche")))
  (return (or (Math|Integer|InRange(Integer) 0 (+ Point (Math|Random|RandomIntegerinRange 4 8)) (+ Point 40)) (Math|Integer|InRange(Integer) 0 (- Point 40) (- Point (Math|Random|RandomIntegerinRange 4 8))))))