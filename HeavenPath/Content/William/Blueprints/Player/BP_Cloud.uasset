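; BP_Cloud is a cloud actor that costs HP through the game mode, then destroys itself.
; On BeginPlay it caches the game mode's Point and the sign of its Angle as right or left.
; Each Tick tests an unwired value against a randomised window on that side of the cached point.
; Every hit calls LostHP and restarts a random retriggerable delay before destruction, with debug prints throughout.
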(event EventBeginPlay
  (bind _asbp_game_mode (Utilities|Casting|CastToBP_GameMode (Game|GetGameMode)))
  (Variables|Default|SetGameMode _asbp_game_mode)
  (Variables|Default|SetPlayerPosition (Variables|/Game/William/Blueprints/Player/BP_GameMode.BP_GameMode_C|GetPoint (Variables|Default|GetGameMode)))
  (Variables|Default|SetIsRight (> (Variables|/Game/William/Blueprints/Player/BP_GameMode.BP_GameMode_C|GetAngle (Variables|Default|GetGameMode)) 0.0)))

(event EventTick
  (params (DeltaSeconds :type Float%20%28single-precision%29))
  (bind _playerposition (Variables|Default|GetPlayerPosition))
  (if (Variables|Default|GetIsRight)
    (Development|PrintString "Droite")
    (if (Math|Integer|InRange(Integer) 0 (+ _playerposition (Math|Random|RandomIntegerinRange 4 8)) (+ _playerposition 40))
      (Default|LostHP (Variables|Default|GetGameMode) :!label _label)
      (Utilities|FlowControl|RetriggerableDelay (Math|Random|RandomFloatinRange 1.0 3.0))
      (Development|PrintString "suicidez-le!")
      (Actor|DestroyActor))
    (else
      (Development|PrintString "gauche")
      (if (Math|Integer|InRange(Integer) 0 (- _playerposition 40) (- _playerposition (Math|Random|RandomIntegerinRange 4 8)))
        (goto _label)))))

(fn ConstructionScript)