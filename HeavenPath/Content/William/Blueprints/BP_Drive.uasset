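; BP_Drive is a steering control with Left and Right parts that adjust a shared angle in BP_GameMode.
; Using picks the side and opens a gate that Tick enters while left mouse is held past a short delay, until Unsing closes it.
; Each pass spins that part, shifts the clamped angle by RotationPower and rotates a decal to match.
; Tick resets both parts' material every frame, so SetActive must be called repeatedly to keep a highlight.
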(event Custom|SetActive
  (params (Target :type Primitive%20Component%20Object%20Reference))
  (Rendering|Material|SetMaterial Target 0 "/Game/FirstPerson/Meshes/FirstPersonProjectileMaterial.FirstPersonProjectileMaterial"))

(event Custom|Using
  (params (TargetHandler :type Actor%20Component%20Object%20Reference))
  (bind _asbp_game_mode (Utilities|Casting|CastToBP_GameMode (Game|GetGameMode)))
  (Variables|Default|SetGameMode _asbp_game_mode)
  (if (== TargetHandler (Variables|Default|GetRight))
    (Variables|Default|SetIsRight true)
    (Utilities|FlowControl|Gate true) ; enters at Open
    (else
      (Variables|Default|SetIsRight false)
      (Utilities|FlowControl|Gate true) ; enters at Open
    )))

(event Custom|Unsing
  (Utilities|FlowControl|Gate true) ; enters at Close
)

(event EventTick
  (params (DeltaSeconds :type Float%20%28single-precision%29))
  (Rendering|Material|SetMaterial (Variables|Default|GetRight) 0 "/Engine/BasicShapes/BasicShapeMaterial.BasicShapeMaterial")
  (if (>= (Class|PlayerController|GetInputKeyTimeDown (Game|GetPlayerController 0) "LeftMouseButton") 0.16)
    (Utilities|FlowControl|Gate true
      (:Exit
        (CallFunction|CalculeAngle (Variables|Default|GetIsRight))
        (if (Variables|Default|GetIsRight)
          (Variables|Default|SetRotationPowerR (+ (Variables|Default|GetRotationPowerR) -2.0))
          (Transformation|SetRelativeRotation (Variables|Default|GetRight) (Math|Rotator|MakeRotator 0.0 (Variables|Default|GetRotationPowerR) 0.0) false false)
          (else
            (Variables|Default|SetRotationPowerL (+ (Variables|Default|GetRotationPowerL) 2.0))
            (Transformation|SetRelativeRotation (Variables|Default|GetLeft) (Math|Rotator|MakeRotator 0.0 (Variables|Default|GetRotationPowerL) 0.0) false false)))))))

(fn ConstructionScript)

(fn CalculeAngle
  (params (Isright :type Boolean))
  (bind _gamemode (Variables|Default|GetGameMode))
  (bind _gamemode_2 (Variables|Default|GetGameMode))
  (if Isright
    (bind _output_get (Variables|/Game/William/Blueprints/Player/BP_GameMode.BP_GameMode_C|SetAngle _gamemode (Math|Float|Clamp(Float) (+ (Variables|/Game/William/Blueprints/Player/BP_GameMode.BP_GameMode_C|GetAngle _gamemode) (Variables|/Game/William/Blueprints/Player/BP_GameMode.BP_GameMode_C|GetRotationPower _gamemode)) -45.0 45.0)))
    (else
      (Variables|/Game/William/Blueprints/Player/BP_GameMode.BP_GameMode_C|SetAngle _gamemode_2 (Math|Float|Clamp(Float) (- (Variables|/Game/William/Blueprints/Player/BP_GameMode.BP_GameMode_C|GetAngle _gamemode_2) (Variables|/Game/William/Blueprints/Player/BP_GameMode.BP_GameMode_C|GetRotationPower _gamemode_2)) -45.0 45.0))))
  (Transformation|SetRelativeRotation (Variables|Default|GetDecal) (Math|Rotator|MakeRotator (+ (* _output_get -1.0) 9e+01) 0.0 9e+01) false false))