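; Interactable cannon that deploys, then fires on the monster when used.
; Deployement plays a timeline that moves the mesh along local Z and, once, caches the first BP_Monster found in the level.
; UsingObject plays a sound, prints charge and fire messages around a short delay, then calls Damage on that monster directly, with a DoOnce blocking reuse until the shot completes.
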(event Custom|Deployement
  (bind _lerp (Timeline|Deploi Play)
    (:Update
      (Transformation|SetRelativeLocation (Variables|Character|GetMesh) (Math|Vector|MakeVector 0.0 0.0 _lerp) false false)
      (Utilities|FlowControl|DoOnce false
        (:Completed
          (bind _outactors (Actor|GetAllActorsOfClass "/Game/William/Blueprints/BP_Monster.BP_Monster_C"))
          (Variables|Default|SetMonster (Utilities|Array|Get(acopy) _outactors)))))))

(event EventTick
  (params (DeltaSeconds :type Float%20%28single-precision%29))
  (|CallParentFunction DeltaSeconds) ; This node is disabled and will not be called.\nDrag off pins to build functionality.
)

(event EventUsingObject
  (Utilities|FlowControl|DoOnce false :!label _label
    (:Completed
      (Audio|SpawnSoundatLocation 0 "0, 0, 0" "0, 0, 0" 1.0 1.0 0.0 "/Game/William/Sound/Bête/AT_Bête.AT_Bête")
      (Development|PrintString "Charge..")
      (Utilities|FlowControl|Delay 2.0)
      (Development|PrintString "Feu!")
      (Default|Damage (Variables|Default|GetMonster))
      (goto _label Reset))))

(fn ConstructionScript
  (|CallParentFunction))