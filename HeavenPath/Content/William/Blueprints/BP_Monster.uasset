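; BP_Monster is a monster encounter staged through positioned sounds and camera shakes, deploying the Interaction_Canon actor after a timed intro.
; A looping attack uses a DoN counter and delays to open a vulnerability window, then costs the game mode HP unless the monster was hit.
; Damage only counts during that window; at zero HP the monster advances BP_Timeline and destroys itself.
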(event Custom|Attaque
  (Utilities|FlowControl|Sequence :!label _label
    (:then_0
      (bind _returnvalue (Audio|SpawnSoundatLocation "/Game/William/Sound/Bête/AttaqueBêteSeq_V1_1.AttaqueBêteSeq_V1_1" (Variables|Default|GetSoundLocation) "0, 0,-90.000000" 15.0 1.0 0.0 "/Game/William/Sound/Bête/AT_Bête.AT_Bête"))
      (bind _output_get (Variables|Default|SetSound _returnvalue))
      (Utilities|FlowControl|Delay 4.0)
      (Utilities|IsValid _output_get
        (:Is%20Valid
          (Audio|Components|Audio|FadeOut _output_get 0.6 0.0 :!class /Script/Engine.AudioComponent))))
    (:then_1
      (bind _counter (Utilities|FlowControl|DoN 6 :!label _label_2)
        (:Exit
          (if (== _counter 6)
            (Variables|Default|SetIsVulnerable false)
            (Utilities|FlowControl|Delay 1.2)
            (if (Variables|Default|GetDamageTake)
              _
              (else
                (Default|LostHP (stale EventBeginPlay _asbp_game_mode) 1e+01)
                (bind _returnvalue_2 (Audio|SpawnSoundatLocation "/Game/William/Sound/Bête/AttaqueLourdeBêteV1_1.AttaqueLourdeBêteV1_1" (Variables|Default|GetSoundLocation) "0, 0,-90.000000" 1e+01 1.0 0.0 "/Game/William/Sound/Bête/AT_Bête.AT_Bête"))
                (Variables|Default|SetSound _returnvalue_2)
                (Camera|PlayWorldCameraShake "/Game/William/Blueprints/BP_camerashake.BP_camerashake_C" (Variables|Default|GetSoundLocation) 0.0 1e+03 1.0 true)))
            (bind _returnvalue_3 (Audio|SpawnSoundatLocation "/Game/William/Sound/Bête/MarcheBêteV1_exemple_.MarcheBêteV1_exemple_" (Variables|Default|GetSoundLocation) "0, 0,-90.000000" 5.0 1.0 0.0 "/Game/William/Sound/Bête/AT_Bête.AT_Bête"))
            (Variables|Default|SetSound _returnvalue_3)
            (Utilities|FlowControl|Delay 5.0)
            (Audio|Components|Audio|FadeOut _returnvalue_3 1.0 0.0 :!class /Script/Engine.AudioComponent)
            (Utilities|FlowControl|Delay 2.0)
            (Variables|Default|SetDamageTake false)
            (Utilities|FlowControl|Sequence
              (:then_0
                (goto _label_2 Reset))
              (:then_1
                (goto _label)))
            (else
              (Variables|Default|SetIsVulnerable true)
              (Utilities|FlowControl|Delay 0.8)
              (goto _label_2))))))))

(event Custom|Damage
  (bind _sound (Variables|Default|GetSound))
  (if (Variables|Default|GetIsVulnerable)
    (Variables|Default|SetDamageTake true)
    (Audio|Components|Audio|Stop (Variables|Default|GetSound))
    (bind _returnvalue (Audio|SpawnSoundatLocation "/Game/William/Sound/Bête/CriBêteDouleurV1.CriBêteDouleurV1" (Variables|Default|GetSoundLocation) "0, 0,-90.000000" 5.0 1.0 0.0 "/Game/William/Sound/Bête/AT_Bête.AT_Bête"))
    (Utilities|FlowControl|Delay 2.0)
    (Audio|Components|Audio|FadeOut _returnvalue 2.0 0.0 :!class /Script/Engine.AudioComponent)
    (Variables|Default|SetHP (- (Variables|Default|GetHP) 1))
    (if (== (Variables|Default|GetHP) 0)
      (Utilities|IsValid _sound
        (:Is%20Valid
          (Audio|Components|Audio|FadeOut _sound 1.0 0.0 :!class /Script/Engine.AudioComponent)
          (Audio|Components|Audio|Stop _sound))
        (:Is%20Not%20Valid
          _))
      (Audio|PlaySoundatLocation "/Game/William/Sound/Bête/CriBêteDouleurV1.CriBêteDouleurV1" (Variables|Default|GetSoundLocation) "0, 0, 0" 8.0 0.8)
      (bind _outactors (Actor|GetAllActorsOfClass "/Game/William/Blueprints/BP_Timeline.BP_Timeline_C"))
      (Variables|/Game/William/Blueprints/BP_Timeline.BP_Timeline_C|SetIndexTab (Utilities|Array|Get(acopy) _outactors) (+ (Variables|/Game/William/Blueprints/BP_Timeline.BP_Timeline_C|GetIndexTab (Utilities|Array|Get(acopy) _outactors)) 1))
      (Default|EventCheck (Utilities|Array|Get(acopy) _outactors))
      (Actor|DestroyActor))))

(event EventBeginPlay
  (bind _asbp_game_mode (Utilities|Casting|CastToBP_GameMode (Game|GetGameMode)))
  (Utilities|FlowControl|Delay 2.0)
  (Camera|PlayWorldCameraShake "/Game/William/Blueprints/BP_camerashake.BP_camerashake_C" (Variables|Default|GetSoundLocation) 0.0 1e+03 1.0 true)
  (Audio|SpawnSoundatLocation "/Game/William/Sound/Bête/MarcheBêteV1_exemple_.MarcheBêteV1_exemple_" (Variables|Default|GetSoundLocation) "0, 0,-90.000000" 5.0 1.0 0.0 "/Game/William/Sound/Bête/AT_Bête.AT_Bête")
  (Utilities|FlowControl|Delay 14.0)
  (Audio|SpawnSoundatLocation "/Game/William/Sound/Bête/CriBête.CriBête" (Variables|Default|GetSoundLocation) "0, 0,-90.000000" 9.0 1.0 0.0 "/Game/William/Sound/Bête/AT_Bête.AT_Bête")
  (Utilities|FlowControl|Delay 2.8)
  (CallFunction|Attaque)
  (bind _outactors (Actor|GetAllActorsOfClass "/Game/William/Blueprints/Interaction_Canon.Interaction_Canon_C"))
  (bind _output_get (Variables|Default|SetCanon (Utilities|Array|Get(acopy) _outactors)))
  (Default|Deployement _output_get))

(fn ConstructionScript)