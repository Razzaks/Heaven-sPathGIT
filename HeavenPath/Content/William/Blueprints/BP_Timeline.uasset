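; BP_Timeline is a scripted sequence actor that spawns clouds and monsters at the player, then quits the game.
; On BeginPlay, EventCheck branches on IndexTab, alternating BP_Cloud and BP_Monster spawns at the player character's transform, with delays before some steps.
; Only the middle pause step increments IndexTab and re-runs EventCheck; spawn steps do not advance the sequence within this Blueprint.
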(event Custom|EventCheck
  (if (== (Variables|Default|GetIndexTab) 0)
    (Utilities|FlowControl|Delay 15.0)
    (CallFunction|CloudEditor)
    (elif (== (Variables|Default|GetIndexTab) 1)
      (Utilities|FlowControl|Delay 1e+01)
      (CallFunction|MonsterEditor)
      (elif (== (Variables|Default|GetIndexTab) 2)
        (Utilities|FlowControl|Delay 1e+01)
        (Variables|Default|SetIndexTab (+ (Variables|Default|GetIndexTab) 1))
        (CallFunction|EventCheck)
        (elif (== (Variables|Default|GetIndexTab) 3)
          (CallFunction|CloudEditor)
          (elif (== (Variables|Default|GetIndexTab) 4)
            (CallFunction|MonsterEditor)
            (elif (== (Variables|Default|GetIndexTab) 5)
              (Utilities|FlowControl|Delay 1e+01)
              (Game|QuitGame 0 "Quit"))))))))

(event EventBeginPlay
  (CallFunction|EventCheck))

(fn ConstructionScript)

(fn CloudEditor
  (Game|SpawnActorfromClass "/Game/William/Blueprints/BP_Cloud.BP_Cloud_C" (Transformation|GetActorTransform (Game|GetPlayerCharacter 0)) "AlwaysSpawn" 0 0))

(fn MonsterEditor
  (Game|SpawnActorfromClass "/Game/William/Blueprints/BP_Monster.BP_Monster_C" (Transformation|GetActorTransform (Game|GetPlayerCharacter 0)) "AlwaysSpawn" 0 0))