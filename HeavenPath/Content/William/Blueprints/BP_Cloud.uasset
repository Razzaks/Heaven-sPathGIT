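; BP_Cloud is a damaging cloud hazard, modelled as a numeric range beside the player's starting GameMode Point, sided by the sign of Angle.
; Each Tick interpolates the range bounds from accumulated time so the zone drifts slightly, then tests the current Point against it.
; Inside, it calls LostHP on BP_GameMode.
; Outside, it calls Nodamage and a Delay-paced counter destroys the actor after roughly ten seconds.
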(event EventBeginPlay
  ;[1 1 1] Begin play
  (bind _asbp_game_mode (Utilities|Casting|CastToBP_GameMode (Game|GetGameMode)))
  (Variables|Default|SetGameMode _asbp_game_mode)
  (Variables|Default|SetPlayerPosition (Math|Float|Truncate (Variables|/Game/William/Blueprints/Player/BP_GameMode.BP_GameMode_C|GetPoint (Variables|Default|GetGameMode))))
  (Variables|Default|SetIsRight (> (Variables|/Game/William/Blueprints/Player/BP_GameMode.BP_GameMode_C|GetAngle (Variables|Default|GetGameMode)) 0.0))
  (Variables|Default|SetVieDanger (Variables|/Game/William/Blueprints/Player/BP_GameMode.BP_GameMode_C|GetHP (Variables|Default|GetGameMode))))

(event EventTick
  (params (DeltaSeconds :type Float%20%28single-precision%29))
  (bind _vitessemov (Variables|Default|GetVitesseMov))
  (bind _gamemode (Variables|Default|GetGameMode))
  (bind _mouvement (Variables|Default|GetMouvement))
  (bind _minrange (Variables|Default|GetMinRange))
  (bind _maxrange (Variables|Default|GetMaxRange))
  ;[1 1 1] Delta time
  (Variables|Default|SetDeltaTime (+ DeltaSeconds (Variables|Default|GetDeltaTime)))
  (if (Math|Float|InRange(Float) (Variables|/Game/William/Blueprints/Player/BP_GameMode.BP_GameMode_C|GetPoint (Variables|Default|GetGameMode)) (Math|Float|SelectFloat (Math|Interpolation|FInterptoConstant (Math|Conversions|ToFloat(Integer) (+ (Variables|Default|GetPlayerPosition) (Math|Integer|SelectInt _minrange (* _minrange -1) (Variables|Default|GetIsRight)))) (Math|Conversions|ToFloat(Integer) (+ (Math|Integer|SelectInt _minrange (* _minrange -1) (Variables|Default|GetIsRight)) (Math|Integer|SelectInt (* _mouvement -1) _mouvement (Variables|Default|GetIsRight)))) (Variables|Default|GetDeltaTime) _vitessemov) (Math|Interpolation|FInterptoConstant (Math|Conversions|ToFloat(Integer) (+ (Variables|Default|GetPlayerPosition) (Math|Integer|SelectInt _maxrange (* _maxrange -1) (Variables|Default|GetIsRight)))) (Math|Conversions|ToFloat(Integer) (+ (Math|Integer|SelectInt _maxrange (* _maxrange -1) (Variables|Default|GetIsRight)) (Math|Integer|SelectInt (* _mouvement -1) _mouvement (Variables|Default|GetIsRight)))) (Variables|Default|GetDeltaTime) _vitessemov) (Variables|Default|GetIsRight)) (Math|Float|SelectFloat (Math|Interpolation|FInterptoConstant (Math|Conversions|ToFloat(Integer) (+ (Variables|Default|GetPlayerPosition) (Math|Integer|SelectInt _maxrange (* _maxrange -1) (Variables|Default|GetIsRight)))) (Math|Conversions|ToFloat(Integer) (+ (Math|Integer|SelectInt _maxrange (* _maxrange -1) (Variables|Default|GetIsRight)) (Math|Integer|SelectInt (* _mouvement -1) _mouvement (Variables|Default|GetIsRight)))) (Variables|Default|GetDeltaTime) _vitessemov) (Math|Interpolation|FInterptoConstant (Math|Conversions|ToFloat(Integer) (+ (Variables|Default|GetPlayerPosition) (Math|Integer|SelectInt _minrange (* _minrange -1) (Variables|Default|GetIsRight)))) (Math|Conversions|ToFloat(Integer) (+ (Math|Integer|SelectInt _minrange (* _minrange -1) (Variables|Default|GetIsRight)) (Math|Integer|SelectInt (* _mouvement -1) _mouvement (Variables|Default|GetIsRight)))) (Variables|Default|GetDeltaTime) _vitessemov) (Variables|Default|GetIsRight)))
    ;[1 1 1] Dégât subit par le nuage
    (Variables|/Game/William/Blueprints/Player/BP_GameMode.BP_GameMode_C|SetIsRight _gamemode (> (Variables|/Game/William/Blueprints/Player/BP_GameMode.BP_GameMode_C|GetAngle _gamemode) 0.0))
    (Variables|Default|SetInCloud true)
    (Default|LostHP (Variables|Default|GetGameMode))
    (Variables|Default|SetVieDanger (Variables|/Game/William/Blueprints/Player/BP_GameMode.BP_GameMode_C|GetHP (Variables|Default|GetGameMode)))
    (Variables|Default|SetTimerSuicide 0.0)
    (else
      ;[1 1 1] Autodestruction du blueprint
      (Utilities|FlowControl|Sequence
        (:then_0
          (Default|Nodamage _gamemode)
          (Utilities|FlowControl|Delay 1.0)
          (Variables|Default|SetTimerSuicide (+ (Variables|Default|GetTimerSuicide) 1.0)))
        (:then_1
          (if (>= (Variables|Default|GetTimerSuicide) 1e+01)
            (Actor|DestroyActor)))))))

(fn ConstructionScript)